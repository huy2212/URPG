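; BP_Player is the player Blueprint, holding two key bindings that act on enemy AI and noise.
; The 1 key finds a single BP_BaseEnemy, casts its controller to AIC_EnemyAIC and uses a FlipFlop to alternate it between attacking and passive states.
; The F key emits a range-limited noise at the player's location, instigated by the player, and spawns an explosion particle effect there.
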(event Input|KeyboardEvents|1
  (params (Key :type Key%20Structure :default "None"))
  (:Pressed
    (bind _returnvalue (Actor|GetActorOfClass "/Game/Blueprints/Enemy/BP_BaseEnemy.BP_BaseEnemy_C"))
    (bind _asaic_enemy_aic (Utilities|Casting|CastToAIC_EnemyAIC (AI|GetAIController _returnvalue)))
    (Utilities|FlowControl|FlipFlop
      (:A
        (Class|EnemyAIController|SetStatetoAttacking _asaic_enemy_aic))
      (:B
        (Class|EnemyAIController|SetStatetoPassive _asaic_enemy_aic)))))

(event Input|KeyboardEvents|F
  (params (Key :type Key%20Structure :default "None"))
  (bind _returnvalue (Transformation|GetActorLocation))
  (:Pressed
    (Class|Actor|MakeNoise 1.0 self _returnvalue 1e+03 "None")
    (Effects|SpawnEmitteratLocation "/Game/ImportedAssets/FXVarietyPack/Particles/P_ky_explosion.P_ky_explosion" _returnvalue)))

(fn ConstructionScript)