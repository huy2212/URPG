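; Base enemy Blueprint that plays the equipped weapon's montages for attacking, blocking, equipping and unequipping.
; Montage notifies during equip and unequip call SpawnWeapon with the right-hand or holder socket, and completion updates IsEquippingWeapon.
; Each action reports back through a Call event when its montage completes, with attack and block also reporting on interruption, unlike equip and unequip.
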(event EventBeginPlay
  ;[1 1 1] Spawn Sword
  (Variables|Default|SetIsEquippingWeapon false))

(event EventAttack
  ;[1 1 1] Attack Event
  (Animation|Montage|PlayMontage (Variables|Character|GetMesh) (Class|Weapon|GetWeaponAttackMontage (Variables|Default|GetEquippedWeapon))
    (:OnCompleted
      _)
    (:OnInterrupted
      _))
  (Default|CallOnAttackEnd))

(event EventEquipWeapon
  ;[1 1 1] Equip Weapon
  (bind _notifyname (Animation|Montage|PlayMontage (Variables|Character|GetMesh) (Class|Weapon|GetWeaponEquipMontage (Variables|Default|GetEquippedWeapon)))
    (:OnCompleted
      (Default|CallOnWeaponEquipped)
      (Variables|Default|SetIsEquippingWeapon true))
    (:OnNotifyBegin
      (switch name _notifyname
        (:UnsheathSword
          (Class|Enemy|SpawnWeapon (Variables|/Script/MyProject.WeaponDataAsset|GetRightHandSocketName (Variables|Default|GetWeaponAsset))))))))

(event EventUnequipWeapon
  ;[1 1 1] Unequip Weapon
  (bind _notifyname (Animation|Montage|PlayMontage (Variables|Character|GetMesh) (Class|Weapon|GetWeaponUnequipMontage (Variables|Default|GetEquippedWeapon)))
    (:OnCompleted
      (Default|CallOnWeaponUnequipeed)
      (Variables|Default|SetIsEquippingWeapon false))
    (:OnNotifyBegin
      (switch name _notifyname
        (:SheathSword
          (Class|Enemy|SpawnWeapon (Variables|/Script/MyProject.WeaponDataAsset|GetHolderSocketName (Variables|Default|GetWeaponAsset))))))))

(event EventPlayBlockMontage
  (Animation|Montage|PlayMontage (Variables|Character|GetMesh) (Class|Weapon|GetWeaponBlockMontage (Variables|Default|GetEquippedWeapon))
    (:OnCompleted
      _)
    (:OnInterrupted
      _))
  (Default|CallOnBlockEnd))

(fn ConstructionScript)