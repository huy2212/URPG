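; BP_RangeEnemy is an enemy Blueprint for a ranged attacker that fires hitscan shots.
; Its Attack event plays the equipped weapon's montage and signals attack end when it completes or is interrupted.
; A montage notify triggers a debug-drawn Visibility line trace from the weapon to the AI controller's attack target.
; Whatever actor the trace hits receives fixed damage through an interface message.
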(event EventBeginPlay
  ;[1 1 1] Spawn Sword
  (Variables|Default|SetIsEquippingWeapon false))

(event EventAttack
  (bind _notifyname (Animation|Montage|PlayMontage (Variables|Character|GetMesh) (Class|Weapon|GetWeaponAttackMontage (Variables|Default|GetEquippedWeapon)) 1.5)
    (:OnCompleted
      (Default|CallOnAttackEnd :!label _label))
    (:OnInterrupted
      (goto _label))
    (:OnNotifyBegin
      (switch name _notifyname
        (:Fire
          (bind _asaic_enemy_aic (Utilities|Casting|CastToAIC_EnemyAIC (AI|GetAIController self)))
          (bind (_outhit _returnvalue) (Collision|LineTraceByChannel (Transformation|GetActorLocation (Variables|Default|GetEquippedWeapon)) (Transformation|GetActorLocation (Class|EnemyAIController|GetAttackTarget _asaic_enemy_aic)) "TraceTypeQuery1" true 0 "ForDuration" true "(R=1.000000,G=0.000000,B=0.000000,A=1.000000)" "(R=0.000000,G=1.000000,B=0.000000,A=1.000000)" 1.0))
          (if _returnvalue
            (Class|HitInterface|TakeDamageInterface(Message) (.HitActor (Collision|BreakHitResult _outhit)) 2e+01 (Utilities|Struct|MakeDamageEvent) 0 self)))))))

(fn ConstructionScript)